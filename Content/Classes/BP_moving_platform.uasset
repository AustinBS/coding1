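; BP_moving_platform is an actor that moves a platform component between a Start and an End point in the world.
; On BeginPlay it hides both endpoint markers and plays a timeline.
; Each timeline update lerps between the two markers' world locations and sets the platform's position without sweep.
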(event EventBeginPlay
  (Rendering|SetVisibility (Variables|Default|Getend) false false)
  (Rendering|SetVisibility (Variables|Default|Getstart) false false)
  (bind _track0 (Timeline|Timeline Play)
    (:Update
      (Transformation|SetWorldLocation (Variables|Default|Getplatform) (Math|Vector|Lerp(Vector) (Transformation|GetWorldLocation (Variables|Default|Getstart)) (Transformation|GetWorldLocation (Variables|Default|Getend)) _track0) false false))))

(fn ConstructionScript)