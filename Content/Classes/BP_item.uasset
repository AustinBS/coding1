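; BP_item is an item actor typed as weapon, tool or consumable that damages an enemy automatically after spawning.
; On BeginPlay, Constructor sets damage by type, rolling it for weapons and picking a random name for unnamed ones.
; It prints both, then after a delay subtracts scaled damage from the Health of the first BP_enemy found.
; BeginPlay also starts a Timeline that moves the Cube vertically.
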(event EventBeginPlay
  (Utilities|FlowControl|Sequence
    (:then_0
      (CallFunction|Constructor)
      (Development|PrintString (Utilities|String|Append "Name: " (Variables|Default|GetName) "Damage: " (Utilities|String|ToString(Integer) (Variables|Default|GetDamage))))
      (Utilities|FlowControl|Delay 5.0)
      (bind _returnvalue (Actor|GetActorOfClass "/Game/Blueprints/BP_enemy.BP_enemy_C"))
      (CallFunction|Attack _returnvalue))
    (:then_1
      (bind _newtrack_0 (Timeline|Timeline Play)
        (:Update
          (Transformation|SetRelativeLocation (Variables|Default|GetCube) (Math|Vector|MakeVector 0.0 0.0 (Math|Float|Lerp 0.0 1e+02 _newtrack_0)) false false))))))

(event Collision|EventActorBeginOverlap
  (params (OtherActor :type Actor%20Object%20Reference)))

(event EventTick
  (params (DeltaSeconds :type Float%20%28single-precision%29)))

(fn ConstructionScript)

(fn Constructor
  (bind _weaponname (Variables|Default|GetweaponName))
  (switch Utilities|FlowControl|Switch|SwitchonitemType (Variables|Default|GetType)
    (:NewEnumerator0
      (Variables|Default|SetDamage (Math|Random|RandomIntegerinRange 3 6))
      (if (Utilities|Enum|Equal(Enum) (Variables|Default|GetName) "")
        (Utilities|Array|Shuffle _weaponname)
        (Variables|Default|SetName (Utilities|Array|Get(acopy) _weaponname))))
    (:NewEnumerator1
      (Variables|Default|SetDamage 1))
    (:NewEnumerator2
      (Variables|Default|SetDamage 0))))

(fn Attack
  (params (givenEnemy :type BP%20Enemy%20Object%20Reference))
  (Variables|/Game/Blueprints/BP_enemy.BP_enemy_C|Sethealth givenEnemy (- (Variables|/Game/Blueprints/BP_enemy.BP_enemy_C|Gethealth givenEnemy) (* (Math|Conversions|ToFloat(Integer) (Variables|Default|GetDamage)) 0.1))))