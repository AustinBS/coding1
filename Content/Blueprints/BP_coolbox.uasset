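; BP_coolbox is an actor with a Cube component that endlessly spawns actors above itself.
; On BeginPlay it prints debug messages with its name, the cube's location and the raised spawn point.
; It then loops through a Delay set by SpawnDelay, spawning an actor at a fixed height above the cube with a random uniform scale each pass.
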(event EventBeginPlay
  (bind _cube (Variables|Default|GetCube))
  (bind _returnvalue (Transformation|GetWorldLocation _cube))
  (bind _returnvalue_2 (+ _returnvalue "0.000000,0.000000,300.000000"))
  (Development|PrintString (Utilities|String|Append (Utilities|GetDisplayName self) " exists!") true true "(R=0.000000,G=0.660000,B=1.000000,A=1.000000)" 1e+01) ; this is cout
  (Development|PrintString (Utilities|String|ToString(Vector) _returnvalue) true true "(R=0.488000,G=0.010248,B=0.010248,A=1.000000)" 1e+01) ; this is cout
  (Development|PrintString (Utilities|String|ToString(Vector) _returnvalue_2) true true "(R=0.878166,G=1.000000,B=0.000000,A=1.000000)" 1e+01)
  (Game|SpawnActorfromClass "/Game/Blueprints/BP_key.BP_key_C" (Math|Transform|MakeTransform _returnvalue_2 "0, 0, 0" (Math|Conversions|ToVector(Float) (Math|Random|RandomFloatinRange 0.5 1e+01))) "Undefined" "MultiplyWithRoot" 0 0 :!label _label)
  (Utilities|FlowControl|Delay (Variables|Default|GetSpawn%20Delay))
  (goto _label))

(fn ConstructionScript)